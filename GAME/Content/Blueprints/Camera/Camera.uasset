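; Camera actor that becomes the player's view target on BeginPlay and tracks the player character.
; Each tick it rotates its camera component toward the pawn and maps their clamped, normalized distance to a lerp between minimum and maximum FOV.
; It then loops over PERSONAGEM actors, printing their locations and moving by Direção: "h" copies the character's Y, while "v" sets X to zero rather than following.
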(event `self.ReceiveBeginPlay`
  (set `self.Personagem` (`GameplayStatics.GetPlayerPawn` 0))
  (`PlayerController.SetViewTargetWithBlend` (`GameplayStatics.GetPlayerController` 0) self 0.0 "VTBlend_Linear" 0.0 false))

(event `self.ReceiveTick`
  (params (DeltaSeconds :type "Float (single-precision)"))
  (`self.AtualizaCamera`)
  (`self.AtualizaDistancia`)
  (`self.NormalizaDistancia`)
  (`self.AtualizaFOV`)
  (`self.AtualizaPosição`))

(fn `AtualizaCamera`
  (bind _cameracomponent (`self.CameraComponent`))
  (`SceneComponent.K2_SetWorldRotation` _cameracomponent (`KismetMathLibrary.FindLookAtRotation` (`SceneComponent.K2_GetComponentLocation` _cameracomponent) (`self.K2_GetActorLocation` (`self.Personagem`))) false false))

(fn `AtualizaDistancia`
  (set `self.Distancia` (`self.GetDistanceTo` (`self.Personagem`))))

(fn `AtualizaFOV`
  (`CameraComponent.SetFieldOfView` (`self.CameraComponent`) (`KismetMathLibrary.Lerp` (`self.FOVMin`) (`self.FOVMax`) (`self.AtualDistancia`))))

(fn `AtualizaPosição`
  (bind `_direção` (`self.Direção`))
  (bind _outactors (`GameplayStatics.GetAllActorsOfClass` "/Game/BLUEPRINTS/Personagem/PERSONAGEM.PERSONAGEM_C"))
  (for _array_element _outactors
    (bind _aspersonagem (cast `/Game/BLUEPRINTS/Personagem/PERSONAGEM` _array_element))
    (bind _returnvalue (`self.K2_GetActorLocation` _aspersonagem))
    (`KismetSystemLibrary.PrintString` (`KismetStringLibrary.Conv_VectorToString` _returnvalue))
    (if (`KismetStringLibrary.EqualEqual_StrStr` `_direção` "h")
      (`self.K2_SetActorLocation` (`KismetMathLibrary.MakeVector` (.x (`self.K2_GetActorLocation`)) (.y _returnvalue) (.z (`self.K2_GetActorLocation`))))
      (elif (`KismetStringLibrary.EqualEqual_StrStr` `_direção` "v")
        (`self.K2_SetActorLocation` (`KismetMathLibrary.MakeVector` 0.0 (.y (`self.K2_GetActorLocation`)) (.z (`self.K2_GetActorLocation`))))))))

(fn `NormalizaDistancia`
  (set `self.AtualDistancia` (`KismetMathLibrary.FClamp` (`KismetMathLibrary.NormalizeToRange` (`self.Distancia`) (`self.DistMin`) (`self.DistMax`)))))

(fn `UserConstructionScript`)